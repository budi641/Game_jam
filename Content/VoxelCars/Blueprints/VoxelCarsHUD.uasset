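; HUD Blueprint for the VoxelCars demo that draws on-screen key hints for switching cars and car colors.
; On each DrawHUD it computes width and height ratios against a 1280x720 reference.
; It then draws the two text lines at positions scaled by those ratios, with text size following the height ratio.
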(event EventDrawHUD
  (params (SizeX :type Integer) (SizeY :type Integer))
  ;[1 1 1] Calculate ratio from 720p
  (Utilities|FlowControl|Sequence
    (:then_0
      (Variables|Default|SetHUDXRatio (/ (Math|Conversions|ToFloat(Integer) SizeX) 1.28e+03)))
    (:then_1
      (Variables|Default|SetHUDYRatio (/ (Math|Conversions|ToFloat(Integer) SizeY) 7.2e+02)))
    (:then_2
      ;[1 1 1] Print texts
      (HUD|DrawText "Keys 1,2,3,4,5 - switch cars" "(R=1.000000,G=1.000000,B=1.000000,A=1.000000)" (* 1e+01 (Variables|Default|GetHUDXRatio)) (* 2e+01 (Variables|Default|GetHUDYRatio)) "/Engine/EngineFonts/RobotoDistanceField.RobotoDistanceField" (* 1.0 (Variables|Default|GetHUDYRatio)) false)
      (HUD|DrawText "Key F - switch car colors" "(R=1.000000,G=1.000000,B=1.000000,A=1.000000)" (* 1e+01 (Variables|Default|GetHUDXRatio)) (* 6e+01 (Variables|Default|GetHUDYRatio)) "/Engine/EngineFonts/RobotoDistanceField.RobotoDistanceField" (* 1.0 (Variables|Default|GetHUDYRatio)) false))))

(fn ConstructionScript)