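; Player controller for the Voxel Cars project that lets the player switch between five voxel car pawns and change their color scheme.
; On BeginPlay it finds the first placed actor of each car class and requests possession of the second car.
; Number keys 1–5 call SwitchPawn, which skips invalid or already selected cars before repossessing through player controller 0.
; The F key cycles the current car's color scheme.
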(event EventBeginPlay
  (bind _outactors (Actor|GetAllActorsOfClass "/Game/VoxelCars/Blueprints/VoxelCar01/VoxelCar01_BP.VoxelCar01_BP_C"))
  (Variables|Default|SetVoxelCar01_Pawn (Utilities|Array|Get(acopy) _outactors))
  (bind _outactors_2 (Actor|GetAllActorsOfClass "/Game/VoxelCars/Blueprints/VoxelCar02/VoxelCar02_BP.VoxelCar02_BP_C"))
  (Variables|Default|SetVoxelCar02_Pawn (Utilities|Array|Get(acopy) _outactors_2))
  (bind _outactors_3 (Actor|GetAllActorsOfClass "/Game/VoxelCars/Blueprints/VoxelCar03/VoxelCar03_BP.VoxelCar03_BP_C"))
  (Variables|Default|SetVoxelCar03_Pawn (Utilities|Array|Get(acopy) _outactors_3))
  (bind _outactors_4 (Actor|GetAllActorsOfClass "/Game/VoxelCars/Blueprints/VoxelCar04/VoxelCar04_BP.VoxelCar04_BP_C"))
  (Variables|Default|SetVoxelCar04_Pawn (Utilities|Array|Get(acopy) _outactors_4))
  (bind _outactors_5 (Actor|GetAllActorsOfClass "/Game/VoxelCars/Blueprints/VoxelCar05/VoxelCar05_BP.VoxelCar05_BP_C"))
  (Variables|Default|SetVoxelCar05_Pawn (Utilities|Array|Get(acopy) _outactors_5))
  ;[1 1 1] Start with VoxelCar02
  (CallFunction|SwitchPawn (Variables|Default|GetVoxelCar02_Pawn) 1))

(event EventTick
  (params (DeltaSeconds :type Float%20%28single-precision%29)))

(event Input|KeyboardEvents|F
  (params (Key :type Key%20Structure))
  (bind _curr_pawn (Variables|Default|GetCurr_Pawn))
  ;[1 1 1] Switch to next color scheme
  (:Pressed
    (Utilities|IsValid _curr_pawn
      (:Is%20Valid
        (Default|SetNextColorScheme _curr_pawn))
      (:Is%20Not%20Valid
        (Development|PrintString "Voxel Cars: Pawn not set!" true true "(R=1.000000,G=0.000000,B=0.000000,A=1.000000)" 5.0)))))

(event Input|KeyboardEvents|1
  (params (Key :type Key%20Structure))
  ;[1 1 1] Switch Car pawns
  (:Pressed
    (CallFunction|SwitchPawn (Variables|Default|GetVoxelCar01_Pawn))))

(event Input|KeyboardEvents|2
  (params (Key :type Key%20Structure))
  ;[1 1 1] Switch Car pawns
  (:Pressed
    (CallFunction|SwitchPawn (Variables|Default|GetVoxelCar02_Pawn) 1)))

(event Input|KeyboardEvents|3
  (params (Key :type Key%20Structure))
  ;[1 1 1] Switch Car pawns
  (:Pressed
    (CallFunction|SwitchPawn (Variables|Default|GetVoxelCar03_Pawn) 2)))

(event Input|KeyboardEvents|4
  (params (Key :type Key%20Structure))
  ;[1 1 1] Switch Car pawns
  (:Pressed
    (CallFunction|SwitchPawn (Variables|Default|GetVoxelCar04_Pawn) 3)))

(event Input|KeyboardEvents|5
  (params (Key :type Key%20Structure))
  ;[1 1 1] Switch Car pawns
  (:Pressed
    (CallFunction|SwitchPawn (Variables|Default|GetVoxelCar05_Pawn) 4)))

(fn ConstructionScript)

(fn SwitchPawn
  (params (Pawn :type BP%20Voxel%20Car%20Base%20Object%20Reference) (Id :type Integer))
  (bind _returnvalue (Game|GetPlayerController 0))
  ;[1 1 1] Just Pawn switcher
  (Utilities|IsValid Pawn
    (:Is%20Valid
      (if (!= Id (Variables|Default|GetCurr_Id))
        (Pawn|UnPossess _returnvalue)
        (Pawn|Possess _returnvalue Pawn)
        (Variables|Default|SetCurr_Id Id)
        (Variables|Default|SetCurr_Pawn Pawn)))
    (:Is%20Not%20Valid
      _))
  (return))